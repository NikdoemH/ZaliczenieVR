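; Game mode for a Beat Saber-style game that spawns flying cubes and tracks the score.
; A looping timer, started on BeginPlay, spawns BP_FlyCube around a TargetPoint, its up-vector offset randomly rolled to left, top or right.
; Each cube's damage event increments the score shown on BP_ScoreText.
; A cube's game-over event destroys all cubes and zeroes the score while spawning continues.
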(event Custom|RestartGame
  (Utilities|Time|ClearandInvalidateTimerbyHandle (Variables|Default|GetCubeSpawnTimerHandle))
  (bind _returnvalue (Utilities|Time|SetTimerbyEvent (delegate Custom|SpawnCube) 2.0 true))
  (Variables|Default|SetCubeSpawnTimerHandle _returnvalue))

(event Custom|SpawnCube
  (bind _cubespawnorgin (Variables|Default|GetCubeSpawnOrgin))
  (bind _returnvalue (Transformation|GetActorTransform _cubespawnorgin))
  (bind _returnvalue_2 (Game|SpawnActorfromClass "/Game/Blueprint/BP_FlyCube.BP_FlyCube_C" (Math|Transform|MakeTransform (+ (.location _returnvalue) (Math|Vector|RotateVector (* (Math|Vector|GetUpVector "0, 0, 0") (Variables|Default|GetSpawnOffset)) (Math|Rotator|MakeRotator (Math|Conversions|ToFloat(Integer) (* (Math|Random|RandomIntegerinRange -1 1) 90)) 0.0 0.0))) (.rotation _returnvalue) "1.000000,1.000000,1.000000") "AlwaysSpawn" "MultiplyWithRoot" 0 0))
  (EventDispatchers|BindEventtoOnTakeAnyDamage _returnvalue_2 (delegate Custom|OnCubeDamage))
  (EventDispatchers|BindEventtoOnGameOver _returnvalue_2 (delegate Custom|OnGameOver)))

(event Custom|OnCubeDamage
  (params (DamagedActor :type Actor%20Object%20Reference) (Damage :type Float%20%28single-precision%29) (DamageType :type Damage%20Type%20Object%20Reference) (InstigatedBy :type Controller%20Object%20Reference) (DamageCauser :type Actor%20Object%20Reference))
  (bind _result (Math|Integer|IncrementInt (Variables|Default|GetScore))
    (:%20%20
      (Default|SetScore (Variables|Default|GetScoreTextActor) _result))))

(event Custom|OnGameOver
  (bind _outactors (Actor|GetAllActorsOfClass "/Game/Blueprint/BP_FlyCube.BP_FlyCube_C"))
  (for _array_element _outactors
    (Actor|DestroyActor _array_element))
  (Variables|Default|SetScore 0)
  (Default|SetScore (Variables|Default|GetScoreTextActor)))

(event EventBeginPlay
  (bind _returnvalue (Actor|GetActorOfClass "/Script/Engine.TargetPoint"))
  (Variables|Default|SetCubeSpawnOrgin _returnvalue)
  (bind _returnvalue_2 (Actor|GetActorOfClass "/Game/Blueprint/BP_ScoreText.BP_ScoreText_C"))
  (Variables|Default|SetScoreTextActor _returnvalue_2)
  (CallFunction|RestartGame))

(event EventTick
  (params (DeltaSeconds :type Float%20%28single-precision%29)))

(fn ConstructionScript)