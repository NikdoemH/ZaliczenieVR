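; BP_LaserSword is a laser sword actor that damages whatever its blade hits.
; BeginPlay caches the mesh's blade socket locations and derives a trace radius from blade length.
; Each Tick runs sphere traces interpolated along the blade toward cached locations, applying damage on every valid hit.
; The cache refreshes inside the loop, so only the first trace spans movement since the previous frame.
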(event Custom|CacheTraceLocations
  (bind _staticmesh (Variables|Default|GetStaticMesh))
  (Variables|Default|SetLastTaceStartLocation (Transformation|GetSocketLocation _staticmesh "TargetStart"))
  (Variables|Default|SetLastTraceEndLocation (Transformation|GetSocketLocation _staticmesh "TargetEnd")))

(event EventBeginPlay
  (CallFunction|CacheTraceLocations)
  (Variables|Default|SetTraceStep (/ (Math|Vector|Distance(Vector) (Variables|Default|GetLastTaceStartLocation) (Variables|Default|GetLastTraceEndLocation)) 2e+01)))

(event EventTick
  (params (DeltaSeconds :type Float%20%28single-precision%29))
  (bind _staticmesh (Variables|Default|GetStaticMesh))
  (for _index (range 0 10)
    (bind _outhit (Collision|SphereTraceByChannel (Math|Vector|Lerp(Vector) (Transformation|GetSocketLocation _staticmesh "TargetStart") (Transformation|GetSocketLocation _staticmesh "TargetEnd") (/ (Math|Conversions|ToFloat(Integer) _index) 1e+01)) (Math|Vector|Lerp(Vector) (Variables|Default|GetLastTaceStartLocation) (Variables|Default|GetLastTraceEndLocation) (/ (Math|Conversions|ToFloat(Integer) _index) 1e+01)) (Variables|Default|GetTraceStep) "TraceTypeQuery1" false 0 "None"))
    (CallFunction|CacheTraceLocations)
    (Utilities|IsValid (.HitActor (Collision|BreakHitResult _outhit))
      (:Is%20Valid
        (Game|Damage|ApplyDamage (.HitActor (Collision|BreakHitResult _outhit)) 1e+02 0 self "/Script/Engine.DamageType")))))

(fn ConstructionScript)